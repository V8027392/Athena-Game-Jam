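; Test enemy that spawns as a Bad, Good or Neutral type, wanders near its spawner and dies to the player's knives.
; BeginPlay rolls a weighted type, falling back when per-type caps on player-held counters are full, then tints the material and starts a looping AI move.
; A knife overlap feeds the player's justice meter, with a sanity event for Neutrals.
; Death updates counters, drops a physics mesh, screams, then destroys the actor.
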(event `Movement`
  (if (not (`self.Dead?`))
    (bind _spawner_ref (`self.Spawner_Ref`)
      (:`then`
        (bind _boxextent_x (`KismetMathLibrary.BreakVector` (`BoxComponent.BoxExtent` (`/Game/Blueprints/Main_Game/Enemy_Spawner.Box` _spawner_ref))))
        (`AIController.MoveToLocation` (`AIBlueprintHelperLibrary.GetAIController` self) (`NavigationSystemV1.K2_GetRandomLocationInNavigableRadius` (`self.K2_GetActorLocation`) _boxextent_x null null) -1.0 true true true true null true)
        (`KismetSystemLibrary.Delay` (`KismetMathLibrary.RandomFloatInRange` 2.0 5.0))
        (`self.Movement`))
      (:`else`
        (`KismetSystemLibrary.Delay` 0.1)
        (`self.Movement`)))))

(event `self.ReceiveBeginPlay`
  (bind _inst_ref (`self.Inst_Ref`))
  (bind _asmain_instance (cast `/Game/Blueprints/Main_Instance` (`GameplayStatics.GetGameInstance`)))
  (set `self.Inst_Ref` _asmain_instance)
  (bind _asmain_character (cast `/Game/Blueprints/Main_Character` (`GameplayStatics.GetPlayerCharacter` 0)))
  (set `self.Player Ref` _asmain_character)
  (`self.Enemy Type Selection`)
  (bind _returnvalue (`PrimitiveComponent.CreateDynamicMaterialInstance` (`self.Cube`) 0 "/Game/Blueprints/Enemies/M_Enemy_Mat.M_Enemy_Mat" "None"))
  (bind _output_get (set `self.Enemy_Mat` _returnvalue))
  (`MaterialInstanceDynamic.SetVectorParameterValue` _output_get "Colour" (select `/Game/Blueprints/Enemies/Enemy_Type` (`self.Enemy Type`) :`NewEnumerator0` (`/Game/Blueprints/Main_Instance.Bad Colour` _inst_ref) :`NewEnumerator1` (`/Game/Blueprints/Main_Instance.Good Colour` _inst_ref) :`NewEnumerator2` (`/Game/Blueprints/Main_Instance.Neutral Colour` _inst_ref)))
  (`self.Movement`))

(event `self.Box.OnComponentBeginOverlap`
  (params (OverlappedComponent :type "PrimitiveComponent Object Reference") (OtherActor :type "Actor Object Reference") (OtherComp :type "PrimitiveComponent Object Reference") (OtherBodyIndex :type Integer) (bFromSweep :type Boolean) (SweepResult :type "HitResult Structure (by ref)"))
  (bind _enemy_type (`self.Enemy Type`))
  (bind _asmain_character (cast `/Game/Blueprints/Main_Character` OtherActor))
  (if (and (or (== OtherComp (`/Game/Blueprints/Main_Character.Knife1` _asmain_character)) (== OtherComp (`/Game/Blueprints/Main_Character.Knife2` _asmain_character)) (== OtherComp (`/Game/Blueprints/Main_Character.Knife3` _asmain_character)) (== OtherComp (`/Game/Blueprints/Main_Character.Knife4` _asmain_character))) (not (`self.Dead?`)))
    (set `self.Dead?` true)
    (`/Game/Blueprints/Main_Character.Justice Meter` _asmain_character _enemy_type)
    (switch `/Game/Blueprints/Enemies/Enemy_Type` _enemy_type
      (:`NewEnumerator0`
        _)
      (:`NewEnumerator1`
        _)
      (:`NewEnumerator2`
        (`/Game/Blueprints/Main_Character.Sanity Event` (`self.Player Ref`) 0.34)))
    (`self.Death`)))

(event `Death`
  (`/Engine/EditorBlueprintResources/StandardMacros.DoOnce` false
    (:`Completed`
      (`/Game/Blueprints/Main_Character.Counter Increment Check` (`self.Player Ref`) (`self.Enemy Type`))
      (set `self.Dead?` true)
      (`/Engine/EditorBlueprintResources/StandardMacros.DecrementInt` (`/Game/Blueprints/Main_Game/Enemy_Spawner.Current` (`self.Spawner_Ref`))
        (:`  `
          (`SceneComponent.SetVisibility` (`self.Cube`) false false)
          (`CharacterMovementComponent.DisableMovement` (`self.CharacterMovement`))
          (bind _returnvalue (`AddComponent|NODE_AddStaticMeshComponent-0` :`RelativeTransform` (`SceneComponent.GetRelativeTransform` (`self.Cube`))))
          (`PrimitiveComponent.SetSimulatePhysics` _returnvalue true)
          (`PrimitiveComponent.SetMaterial` _returnvalue 0 (`self.Enemy_Mat`))
          (`GameplayStatics.PlaySound2D` "/Game/SFX/Scream1_Cue.Scream1_Cue" 1.0 1.0 0.0 null null)
          (`KismetSystemLibrary.Delay` 2.0)
          (`self.K2_DestroyActor`))))))

(fn `Enemy Type Selection`
  (locals (`Maximum Good/Evil` :type Integer :default 80) (`Maximum Neutral` :type Integer :default 40))
  (bind _player_ref (`self.Player Ref`))
  (bind _player_ref_2 (`self.Player Ref`))
  (bind _player_ref_3 (`self.Player Ref`))
  (bind _player_ref_4 (`self.Player Ref`))
  (bind _player_ref_5 (`self.Player Ref`))
  (bind _player_ref_6 (`self.Player Ref`))
  (bind _player_ref_7 (`self.Player Ref`))
  (bind _player_ref_8 (`self.Player Ref`))
  (bind _player_ref_9 (`self.Player Ref`))
  (bind _output_get (set `self.Enemy Type Selected` (`KismetMathLibrary.RandomIntegerInRange` 0 99)))
  (if (<= _output_get 39)
    (if (>= (`/Game/Blueprints/Main_Character.Bad (Debug)` (`self.Player Ref`)) (`local.Maximum Good/Evil`))
      (if (>= (`/Game/Blueprints/Main_Character.Good (Debug)` (`self.Player Ref`)) (`local.Maximum Good/Evil`))
        (if (>= (`/Game/Blueprints/Main_Character.Neutral (Debug)` (`self.Player Ref`)) (`local.Maximum Neutral`))
          (`KismetSystemLibrary.PrintString` "200 Spawned" true true (struct :`A` 1.0))
          (else
            (set `self.Enemy Type` "NewEnumerator2")
            (set `/Game/Blueprints/Main_Character.Neutral (Debug)` (+ (`/Game/Blueprints/Main_Character.Neutral (Debug)` _player_ref_4) 1) _player_ref_4)))
        (else
          (set `self.Enemy Type` "NewEnumerator1")
          (set `/Game/Blueprints/Main_Character.Good (Debug)` (+ (`/Game/Blueprints/Main_Character.Good (Debug)` _player_ref_3) 1) _player_ref_3)))
      (else
        (set `self.Enemy Type` "NewEnumerator0")
        (set `/Game/Blueprints/Main_Character.Bad (Debug)` (+ (`/Game/Blueprints/Main_Character.Bad (Debug)` _player_ref_5) 1) _player_ref_5)))
    (elif (<= _output_get 79)
      (if (>= (`/Game/Blueprints/Main_Character.Good (Debug)` (`self.Player Ref`)) (`local.Maximum Good/Evil`))
        (if (>= (`/Game/Blueprints/Main_Character.Bad (Debug)` (`self.Player Ref`)) (`local.Maximum Good/Evil`))
          (if (>= (`/Game/Blueprints/Main_Character.Neutral (Debug)` (`self.Player Ref`)) (`local.Maximum Neutral`))
            (`KismetSystemLibrary.PrintString` "200 Spawned" true true (struct :`A` 1.0))
            (else
              (set `self.Enemy Type` "NewEnumerator2")
              (set `/Game/Blueprints/Main_Character.Neutral (Debug)` (+ (`/Game/Blueprints/Main_Character.Neutral (Debug)` _player_ref_6) 1) _player_ref_6)))
          (else
            (set `self.Enemy Type` "NewEnumerator0")
            (set `/Game/Blueprints/Main_Character.Bad (Debug)` (+ (`/Game/Blueprints/Main_Character.Bad (Debug)` _player_ref_7) 1) _player_ref_7)))
        (else
          (set `self.Enemy Type` "NewEnumerator1")
          (set `/Game/Blueprints/Main_Character.Good (Debug)` (+ (`/Game/Blueprints/Main_Character.Good (Debug)` _player_ref_8) 1) _player_ref_8)))
      (elif (>= _output_get 80)
        (if (>= (`/Game/Blueprints/Main_Character.Neutral (Debug)` (`self.Player Ref`)) (`local.Maximum Neutral`))
          (if (>= (`/Game/Blueprints/Main_Character.Bad (Debug)` (`self.Player Ref`)) (`local.Maximum Good/Evil`))
            (if (>= (`/Game/Blueprints/Main_Character.Good (Debug)` (`self.Player Ref`)) (`local.Maximum Good/Evil`))
              (`KismetSystemLibrary.PrintString` "200 Spawned" true true (struct :`A` 1.0))
              (else
                (set `self.Enemy Type` "NewEnumerator1")
                (set `/Game/Blueprints/Main_Character.Good (Debug)` (+ (`/Game/Blueprints/Main_Character.Good (Debug)` _player_ref) 1) _player_ref)))
            (else
              (set `self.Enemy Type` "NewEnumerator0")
              (set `/Game/Blueprints/Main_Character.Bad (Debug)` (+ (`/Game/Blueprints/Main_Character.Bad (Debug)` _player_ref_9) 1) _player_ref_9)))
          (else
            (set `self.Enemy Type` "NewEnumerator2")
            (set `/Game/Blueprints/Main_Character.Neutral (Debug)` (+ (`/Game/Blueprints/Main_Character.Neutral (Debug)` _player_ref_2) 1) _player_ref_2)))))))

(fn `UserConstructionScript`
  (`PrimitiveComponent.SetMaterial` (`self.Cube`) 0 (select `/Game/Blueprints/Enemies/Enemy_Type` (`self.Enemy Type`) :`NewEnumerator0` "/Game/Blueprints/Enemies/MI_Bad_Mat.MI_Bad_Mat" :`NewEnumerator1` "/Game/Blueprints/Enemies/MI_Good_Mat.MI_Good_Mat" :`NewEnumerator2` "/Game/Blueprints/Enemies/MI_Neutral_Mat.MI_Neutral_Mat" :!type "MaterialInterface Object Reference")))