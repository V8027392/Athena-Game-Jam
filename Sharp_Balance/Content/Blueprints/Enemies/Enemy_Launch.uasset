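; Enemy_Launch is a short-lived enemy actor that is launched upward with random sideways drift and destroys itself three seconds later.
; On BeginPlay it tints its mesh through a dynamic material instance, choosing the Bad, Good or Neutral colour from the Main_Instance game instance by EnemyType.
; ProjectileMovement then supplies the randomised launch velocity.
; All of this depends on the game instance cast succeeding.
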(event `self.ReceiveBeginPlay`
  (bind _returnvalue (`KismetMathLibrary.RandomFloatInRange` -300.0 300.0))
  (bind _inst_ref (`self.Inst_Ref`))
  (bind _asmain_instance (cast `/Game/Blueprints/Main_Instance` (`GameplayStatics.GetGameInstance`)))
  (set `self.Inst_Ref` _asmain_instance)
  (bind _returnvalue_2 (`PrimitiveComponent.CreateDynamicMaterialInstance` (`self.Enemy`) 0 "/Game/Blueprints/Enemies/M_Enemy_Mat.M_Enemy_Mat" "None"))
  (bind _output_get (set `self.Enemy_Mat` _returnvalue_2))
  (`MaterialInstanceDynamic.SetVectorParameterValue` _output_get "Colour" (select `/Game/Blueprints/Enemies/Enemy_Type` (`self.Enemy Type`) :`NewEnumerator0` (`/Game/Blueprints/Main_Instance.Bad Colour` _inst_ref) :`NewEnumerator1` (`/Game/Blueprints/Main_Instance.Good Colour` _inst_ref) :`NewEnumerator2` (`/Game/Blueprints/Main_Instance.Neutral Colour` _inst_ref)))
  (`ProjectileMovementComponent.SetVelocityInLocalSpace` (`self.ProjectileMovement`) (`KismetMathLibrary.MakeVector` _returnvalue _returnvalue 400.0))
  (`KismetSystemLibrary.Delay` 3.0)
  (`self.K2_DestroyActor`))

(fn `UserConstructionScript`)