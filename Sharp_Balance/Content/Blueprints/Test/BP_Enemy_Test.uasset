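; BP_Enemy_Test is a test enemy of random Bad, Good or Neutral type, coloured to match through a dynamic material.
; It loops between random navigable points, using a radius from its spawner's box, with random pauses.
; A player knife overlap shifts Sanity down, up or randomly by type and triggers death.
; Death decrements the spawner's count, swaps the visible cube for a physics-simulated mesh, then destroys the actor after a delay.
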(event `Movement`
  (if (not (`self.Dead?`))
    (bind _spawner_ref (`self.Spawner_Ref`)
      (:`then`
        (bind _boxextent_x (`KismetMathLibrary.BreakVector` (`BoxComponent.BoxExtent` (`/Game/Blueprints/Main_Game/Enemy_Spawner.Box` _spawner_ref))))
        (`AIController.MoveToLocation` (`AIBlueprintHelperLibrary.GetAIController` self) (`NavigationSystemV1.K2_GetRandomLocationInNavigableRadius` (`self.K2_GetActorLocation`) _boxextent_x null null) -1.0 true true true true null true)
        (`KismetSystemLibrary.Delay` (`KismetMathLibrary.RandomFloatInRange` 2.0 5.0))
        (`self.Movement`))
      (:`else`
        (`KismetSystemLibrary.Delay` 0.1)
        (`self.Movement`)))))

(event `self.ReceiveBeginPlay`
  (bind _inst_ref (`self.Inst_Ref`))
  (bind _asmain_instance (cast `/Game/Blueprints/Main_Instance` (`GameplayStatics.GetGameInstance`)))
  (set `self.Inst_Ref` _asmain_instance)
  (set `self.Enemy Type` (select `int` (`KismetMathLibrary.RandomIntegerInRange` 0 2) :`0` "NewEnumerator0" :`1` "NewEnumerator1" :`2` "NewEnumerator2" :!type "/Game/Blueprints/Test/Enemy_Type Enum"))
  (bind _returnvalue (`PrimitiveComponent.CreateDynamicMaterialInstance` (`self.Cube`) 0 "/Game/Blueprints/Test/M_Enemy_Mat.M_Enemy_Mat" "None"))
  (bind _output_get (set `self.Enemy_Mat` _returnvalue))
  (`MaterialInstanceDynamic.SetVectorParameterValue` _output_get "Colour" (select `/Game/Blueprints/Test/Enemy_Type` (`self.Enemy Type`) :`NewEnumerator0` (`/Game/Blueprints/Main_Instance.Bad Colour` _inst_ref) :`NewEnumerator1` (`/Game/Blueprints/Main_Instance.Good Colour` _inst_ref) :`NewEnumerator2` (`/Game/Blueprints/Main_Instance.Neutral Colour` _inst_ref)))
  (`self.Movement`))

(event `self.Box.OnComponentBeginOverlap`
  (params (OverlappedComponent :type "PrimitiveComponent Object Reference") (OtherActor :type "Actor Object Reference") (OtherComp :type "PrimitiveComponent Object Reference") (OtherBodyIndex :type Integer) (bFromSweep :type Boolean) (SweepResult :type "HitResult Structure (by ref)"))
  (bind _asmain_character (cast `/Game/Blueprints/Main_Character` OtherActor))
  (if (== OtherComp (`/Game/Blueprints/Main_Character.Knife` _asmain_character))
    (set `/Game/Blueprints/Main_Character.Sanity` (`KismetMathLibrary.FClamp` (+ (`/Game/Blueprints/Main_Character.Sanity` _asmain_character) (select `/Game/Blueprints/Test/Enemy_Type` (`self.Enemy Type`) :`NewEnumerator0` -0.1 :`NewEnumerator1` 0.1 :`NewEnumerator2` (`KismetMathLibrary.SelectFloat` -0.3 0.3 (`KismetMathLibrary.RandomBool`))))) _asmain_character)
    (`self.Death`)))

(event `Death`
  (`/Engine/EditorBlueprintResources/StandardMacros.DoOnce` false
    (:`Completed`
      (set `self.Dead?` true)
      (`/Engine/EditorBlueprintResources/StandardMacros.DecrementInt` (`/Game/Blueprints/Main_Game/Enemy_Spawner.Current` (`self.Spawner_Ref`))
        (:`  `
          (`SceneComponent.SetVisibility` (`self.Cube`) false false)
          (`CharacterMovementComponent.DisableMovement` (`self.CharacterMovement`))
          (bind _returnvalue (`AddComponent|NODE_AddStaticMeshComponent-0` :`RelativeTransform` (`SceneComponent.GetRelativeTransform` (`self.Cube`))))
          (`PrimitiveComponent.SetSimulatePhysics` _returnvalue true)
          (`PrimitiveComponent.SetMaterial` _returnvalue 0 (`self.Enemy_Mat`))
          (`KismetSystemLibrary.Delay` 2.0)
          (`self.K2_DestroyActor`))))))

(fn `UserConstructionScript`
  (`PrimitiveComponent.SetMaterial` (`self.Cube`) 0 (select `/Game/Blueprints/Test/Enemy_Type` (`self.Enemy Type`) :`NewEnumerator0` "/Game/Blueprints/Test/MI_Bad_Mat.MI_Bad_Mat" :`NewEnumerator1` "/Game/Blueprints/Test/MI_Good_Mat.MI_Good_Mat" :`NewEnumerator2` "/Game/Blueprints/Test/MI_Neutral_Mat.MI_Neutral_Mat" :!type "MaterialInterface Object Reference")))