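; Player character that moves on input axes and scores knife hits on enemies.
; BeginPlay adds the Main_HUD widget, and Tick prints TotalKills as debug output.
; Knife overlaps with BP_Enemy_Test pick a value by EnemyType, negative for Neutral, increment it and overwrite TotalKills rather than accumulating.
; A blood-overlay score-multiplier idea and a timeline-driven knife spin are present but never run.
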(event `self.ReceiveBeginPlay`
  (bind _returnvalue (`|CreateWidget` "/Game/UI/Game/Main_HUD.Main_HUD_C"))
  (bind _output_get (set `self.HUD Ref` _returnvalue))
  (`UserWidget.AddToViewport` _output_get 0))

(event `InputAxis|Move Forward`
  (params (AxisValue :type "Float (single-precision)"))
  (`self.AddMovementInput` (`self.X Value (Movement)`) (* AxisValue 20.0)))

(event `InputAxis|Move Right`
  (params (AxisValue :type "Float (single-precision)"))
  (`self.AddMovementInput` (`self.Y Value (Movement)`) (* AxisValue 20.0)))

(event `self.ReceiveTick`
  (params (DeltaSeconds :type "Float (single-precision)"))
  (`KismetSystemLibrary.PrintString` (`KismetStringLibrary.Conv_IntToString` (stale `self.Knife.OnComponentBeginOverlap` _output_get))))

(event `self.Knife.OnComponentBeginOverlap`
  (params (OverlappedComponent :type "PrimitiveComponent Object Reference") (OtherActor :type "Actor Object Reference") (OtherComp :type "PrimitiveComponent Object Reference") (OtherBodyIndex :type Integer) (bFromSweep :type Boolean) (SweepResult :type "HitResult Structure (by ref)"))
  (bind _asbp_enemy_test (cast `/Game/Blueprints/Test/BP_Enemy_Test` OtherActor))
  (bind _result (`/Engine/EditorBlueprintResources/StandardMacros.IncrementInt` (select `/Game/Blueprints/Test/Enemy_Type` (`/Game/Blueprints/Test/BP_Enemy_Test.Enemy Type` _asbp_enemy_test) :`NewEnumerator0` 1 :`NewEnumerator1` 1 :`NewEnumerator2` -1))
    (:`  `
      (bind _output_get (set `self.Total Kills` _result)))))

(fn `UserConstructionScript`)