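; Main menu pedestal that displays a character for one enemy type (Bad, Good or Neutral, labelled "Citizen") with a text label and a selection widget.
; Construction sets the label and its size from the type and TextSize.
; BeginPlay creates a dynamic material, links the widget back to the pedestal and applies a default colour per type through UpdateMaterial, which maps an index to a palette colour.
; A character rotation timeline exists but never runs.
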(event `self.ReceiveBeginPlay`
  (bind _returnvalue (`PrimitiveComponent.CreateDynamicMaterialInstance` (`self.Character`) 0 "/Game/Blueprints/Test/M_Enemy_Mat.M_Enemy_Mat" "None"))
  (set `self.Enemy_Mat` _returnvalue)
  (bind _returnvalue_2 (`|CreateWidget` "/Game/UI/Main_Menu/Pedestal_Widget.Pedestal_Widget_C"))
  (bind _output_get (set `self.Selection Widget Ref` _returnvalue_2))
  (set `/Game/UI/Main_Menu/Pedestal_Widget.Pedestal Ref` self _output_get)
  (`WidgetComponent.SetWidget` (`self.Widget`) _output_get)
  (bind _output_get_2 (set `self.Int` (select `/Game/Blueprints/Test/Enemy_Type` (`self.Enemy Type`) :`NewEnumerator1` 3 :`NewEnumerator2` 5)))
  (`self.Update Material` _output_get_2))

(event `Update Material`
  (params (Int :type Integer))
  (`MaterialInstanceDynamic.SetVectorParameterValue` (`self.Enemy_Mat`) "Colour" (select `int` Int :`0` (struct :`R` 1.0 :`A` 1.0) :`1` (struct :`R` 1.0 :`G` 0.175515 :`A` 1.0) :`2` (struct :`R` 1.0 :`G` 0.765318 :`A` 1.0) :`3` (struct :`R` 0.053933 :`G` 1.0 :`A` 1.0) :`4` (struct :`G` 1.0 :`B` 0.974876 :`A` 1.0) :`5` (struct :`R` 0.028321 :`B` 1.0 :`A` 1.0) :`6` (struct :`R` 0.477403 :`B` 1.0 :`A` 1.0) :`7` (struct :`R` 1.0 :`B` 0.944171 :`A` 1.0) :`8` (struct :`R` 0.255208 :`G` 0.049435 :`A` 1.0) :!type "LinearColor Structure")))

(fn `UserConstructionScript`
  (bind _text (`self.Text`))
  (`TextRenderComponent.K2_SetText` _text (select `/Game/Blueprints/Test/Enemy_Type` (`self.Enemy Type`) :`NewEnumerator0` (`|FormatText` "Bad") :`NewEnumerator1` (`|FormatText` "Good") :`NewEnumerator2` (`|FormatText` "Citizen")))
  (`TextRenderComponent.SetWorldSize` _text (`self.Text Size`)))