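; Confirm_Selection is a main menu Blueprint, referred to as a sticky note, that hosts a confirm-selection widget and a fadeable Sign.
; On BeginPlay it creates a dynamic unlit material on the Sign at zero opacity, then assigns a new Confirm_Select_Widget, holding a back-reference to itself, to its widget component.
; The Clashing event plays a timeline that drives the material's opacity, apparently as a colour-clash indicator.
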(event `self.ReceiveBeginPlay`
  (bind _returnvalue (`PrimitiveComponent.CreateDynamicMaterialInstance` (`self.Sign`) 0 "/Game/Blueprints/Main_Game/Unlit_Mat.Unlit_Mat" "None"))
  (bind _output_get (set `self.Mat` _returnvalue))
  (`MaterialInstanceDynamic.SetScalarParameterValue` _output_get "Opacity" 0.0)
  (bind _returnvalue_2 (`|CreateWidget` "/Game/UI/Main_Menu/Confirm_Select_Widget.Confirm_Select_Widget_C"))
  (set `/Game/UI/Main_Menu/Confirm_Select_Widget.Sticky Note Ref` self _returnvalue_2)
  (bind _output_get_2 (set `self.Back From Select Widget` _returnvalue_2))
  (`WidgetComponent.SetWidget` (`self.Widget`) _output_get_2))

(event `Clashing`
  (bind (_direction _alpha) (`Timeline|Colour Clash Timeline` :!via `PlayFromStart`)
    (:`Update`
      (`MaterialInstanceDynamic.SetScalarParameterValue` (`self.Mat`) "Opacity" (`KismetMathLibrary.Lerp` 0.0 1.0 _alpha)))))

(fn `UserConstructionScript`)