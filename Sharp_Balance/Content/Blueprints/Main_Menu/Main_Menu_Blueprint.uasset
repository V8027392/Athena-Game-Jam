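; Main menu actor that hosts the menu widget and animates a 3D knife as the selection pointer.
; The widget receives a reference back to this actor on BeginPlay.
; Timelines glide the knife to the hovered option's marker, or raise and drop it onto the hit marker, with a Selected flag blocking input during the strike.
; StartGame blends the player's view to actors tagged "Select".
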(event `self.ReceiveBeginPlay`
  (bind _returnvalue (`|CreateWidget` "/Game/UI/Main_Menu/Main_Menu_Widget.Main_Menu_Widget_C"))
  (set `/Game/UI/Main_Menu/Main_Menu_Widget.Main_Menu_Blueprint_Ref` self _returnvalue)
  (bind _output_get (set `self.Menu_Widget_Ref` _returnvalue))
  (`WidgetComponent.SetWidget` (`self.Main_Menu`) _output_get))

(event `Start Game`
  (bind _outactors (`GameplayStatics.GetAllActorsWithTag` "Select"))
  (for _array_element _outactors
    (`PlayerController.SetViewTargetWithBlend` (`GameplayStatics.GetPlayerController` 0) _array_element 1.0 "VTBlend_Linear" 0.0 false)))

(event `Hover Update`
  (params (Interger :type Integer))
  (bind _knife (`self.Knife`))
  (bind _returnvalue (select `int` Interger :`0` (`self.Start Hover`) :`1` (`self.Settings Hover`) :`2` (`self.Credits Hover`) :`3` (`self.Quit Hover`) :`4` (`self.About Hover`) :!type "SceneComponent Object Reference"))
  (if (not (`self.Selected`))
    (set `self.Knife Current Loc` (`SceneComponent.K2_GetComponentLocation` _knife))
    (set `self.Knife Current Rot` (`SceneComponent.K2_GetComponentRotation` _knife))
    (bind (_direction _alpha) (`Timeline|Movement` :!via `PlayFromStart`)
      (:`Update`
        (`SceneComponent.K2_SetWorldLocation` (`self.Knife`) (`KismetMathLibrary.VLerp` (`self.Knife Current Loc`) (`SceneComponent.K2_GetComponentLocation` _returnvalue) _alpha) false false)
        (`SceneComponent.K2_SetRelativeRotation` (`self.Knife`) (`KismetMathLibrary.RLerp` (`self.Knife Current Rot`) (`KismetMathLibrary.MakeRotator` (.roll (`SceneComponent.K2_GetComponentRotation` _returnvalue)) (.pitch (`SceneComponent.K2_GetComponentRotation` _returnvalue)) (.yaw (`SceneComponent.K2_GetComponentRotation` _returnvalue))) _alpha true) false false)))))

(event `Hit`
  (params (Interget :type Integer))
  (bind _knife (`self.Knife`))
  (bind _returnvalue (select `int` Interget :`0` (`self.Start Hit`) :`1` (`self.Settings Hit`) :`2` (`self.Credits Hit`) :`3` (`self.Quit Game Hit`) :`4` (`self.About Hit`) :!type "SceneComponent Object Reference"))
  (if (not (`self.Selected`))
    (set `self.Selected` true)
    (bind _output_get (set `self.Knife Current Loc` (`SceneComponent.K2_GetComponentLocation` _knife)))
    (set `self.Knife Current Rot` (`SceneComponent.K2_GetComponentRotation` _knife))
    (set `self.Knife Raise` (+ _output_get (0.0 0.0 30.0)))
    (bind (_direction _raise) (`Timeline|Raise` :!via `PlayFromStart`)
      (:`Update`
        (`SceneComponent.K2_SetWorldLocation` (`self.Knife`) (`KismetMathLibrary.VLerp` (`self.Knife Current Loc`) (`self.Knife Raise`) _raise) false false))
      (:`Finished`
        (bind (_direction_2 _alpha) (`Timeline|Drop` :!via `PlayFromStart`)
          (:`Update`
            (`SceneComponent.K2_SetWorldRotation` (`self.Knife`) (`KismetMathLibrary.RLerp` (`self.Knife Current Rot`) (`SceneComponent.K2_GetComponentRotation` _returnvalue) _alpha true) false false)
            (`SceneComponent.K2_SetWorldLocation` (`self.Knife`) (`KismetMathLibrary.VLerp` (`self.Knife Raise`) (`SceneComponent.K2_GetComponentLocation` _returnvalue) _alpha) false false))
          (:`Finished`
            (set `self.Selected` false)))))))

(fn `UserConstructionScript`)