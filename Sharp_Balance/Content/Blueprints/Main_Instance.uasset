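; Main_Instance Blueprint that validates the colours chosen on Pedestal actors for the Bad, Good and Neutral enemy types.
; SelectionCheck reads each pedestal's "Colour" material parameter, stores it as that type's colour and rebuilds ColoursArray.
; A nested pairwise comparison then sets and returns Failed as true if any two pedestals share exactly the same colour.
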(fn `Selection Check`
  (returns (`Has Failed?` :type Boolean))
  (locals (`Colours Array` :type "Array of LinearColor Structure") (`Failed?` :type Boolean))
  (set `local.Failed?` false)
  (`KismetArrayLibrary.Array_Clear` (`local.Colours Array`))
  (bind _outactors (`GameplayStatics.GetAllActorsOfClass` "/Game/Blueprints/Main_Menu/Pedestal.Pedestal_C"))
  (for _array_element _outactors
    (bind _returnvalue (`MaterialInstanceDynamic.K2_GetVectorParameterValue` (`/Game/Blueprints/Main_Menu/Pedestal.Enemy_Mat` _array_element) "Colour"))
    (switch `/Game/Blueprints/Enemies/Enemy_Type` (`/Game/Blueprints/Main_Menu/Pedestal.Enemy Type` _array_element)
      (:`NewEnumerator0`
        (bind _output_get (set `self.Bad Colour` _returnvalue))
        (`KismetArrayLibrary.Array_Add` (`local.Colours Array`) _output_get))
      (:`NewEnumerator1`
        (bind _output_get_2 (set `self.Good Colour` _returnvalue))
        (`KismetArrayLibrary.Array_Add` (`local.Colours Array`) _output_get_2))
      (:`NewEnumerator2`
        (bind _output_get_3 (set `self.Neutral Colour` _returnvalue))
        (`KismetArrayLibrary.Array_Add` (`local.Colours Array`) _output_get_3))))
  (for (_array_element_2 _array_index) (`local.Colours Array`)
    (for (_array_element_3 _array_index_2) (`local.Colours Array`)
      (if (== _array_index_2 _array_index)
        _
        (elif (== _array_element_3 _array_element_2)
          (set `local.Failed?` true)))))
  (return (`local.Failed?`)))