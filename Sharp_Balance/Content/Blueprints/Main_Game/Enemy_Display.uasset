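; Display actor for an enemy mesh that shows its type (Bad, Good, Neutral or Empty) through colour.
; On BeginPlay it creates a dynamic instance of M_Enemy_Mat and sets its Colour parameter from the matching Main_Instance colour, or transparent black for Empty.
; A Rotate timeline for spinning the mesh through a full roll is present but never triggered.
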(event `self.ReceiveBeginPlay`
  (bind _asmain_instance (cast `/Game/Blueprints/Main_Instance` (`GameplayStatics.GetGameInstance`)))
  (bind _returnvalue (`PrimitiveComponent.CreateDynamicMaterialInstance` (`self.Enemy`) 0 "/Game/Blueprints/Enemies/M_Enemy_Mat.M_Enemy_Mat" "None"))
  (bind _output_get (set `self.Enemy_Mat` _returnvalue))
  (`MaterialInstanceDynamic.SetVectorParameterValue` _output_get "Colour" (select `/Game/Blueprints/Enemies/Enemy_Type` (`self.Enemy Type`) :`NewEnumerator0` (`/Game/Blueprints/Main_Instance.Bad Colour` _asmain_instance) :`NewEnumerator1` (`/Game/Blueprints/Main_Instance.Good Colour` _asmain_instance) :`NewEnumerator2` (`/Game/Blueprints/Main_Instance.Neutral Colour` _asmain_instance))))

(fn `UserConstructionScript`)