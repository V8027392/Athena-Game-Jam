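; Blood splat actor that places itself on the surface below, fades through its opacity and then destroys itself.
; On BeginPlay it traces down against WorldStatic objects and moves to the hit location.
; Its four components get random horizontal scales with a fixed flattened height and share one dynamic instance of an unlit material.
; The Fade timeline drives that material's Opacity parameter and destroys the actor when finished.
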(event `self.ReceiveBeginPlay`
  (bind _returnvalue (`SceneComponent.K2_GetComponentLocation` (`self.Cylinder`)))
  (bind _returnvalue_2 (`KismetMaterialLibrary.CreateDynamicMaterialInstance` "/Game/Blueprints/Main_Game/Unlit_Mat.Unlit_Mat"))
  (set `self.Blood` _returnvalue_2)
  (bind _outhit (`KismetSystemLibrary.LineTraceSingleForObjects` _returnvalue (- _returnvalue (0.0 0.0 300.0)) (`|MakeArray` "ObjectTypeQuery1" :!type "EObjectTypeQuery Enum") true))
  (`self.K2_SetActorLocation` (`.Location` (`GameplayStatics.BreakHitResult` _outhit)))
  (for _array_element (`|MakeArray` (`self.Cylinder`) (`self.w`) (`self.w1`) (`self.w2`))
    (bind _output_get (set `self.Scale` (`KismetMathLibrary.RandomFloatInRange` 1.0 3.0)))
    (`SceneComponent.SetRelativeScale3D` _array_element (`KismetMathLibrary.MakeVector` _output_get _output_get 0.6))
    (`PrimitiveComponent.SetMaterial` _array_element 0 (`self.Blood`)))
  (bind (_direction _alpha) (`Timeline|Fade` :!via `PlayFromStart`)
    (:`Update`
      (`MaterialInstanceDynamic.SetScalarParameterValue` (`self.Blood`) "Opacity" _alpha))
    (:`Finished`
      (`self.K2_DestroyActor`))))

(fn `UserConstructionScript`)